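; BP_Char_Corgi is a corgi character that follows the player's TopDownCharacter.
; On BeginPlay it casts and caches the player character at index 0.
; Every Tick it issues a SimpleMoveToActor through its controller toward that character.
; It also stores the distance moved since the previous tick in DeltaDistance, which nothing in this graph reads.
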(event `self.ReceiveBeginPlay`
  (bind _astop_down_character (cast `/Game/TopDownBP/Blueprints/TopDownCharacter` (`GameplayStatics.GetPlayerCharacter` 0)))
  (set `self.As Top Down Character` _astop_down_character))

(event `self.ReceiveTick`
  (params (DeltaSeconds :type "Float (single-precision)"))
  (bind _returnvalue (`self.K2_GetActorLocation` self))
  (`AIBlueprintHelperLibrary.SimpleMoveToActor` (`self.GetController` self) (`self.As Top Down Character`))
  (set `self.DeltaDistance` (`KismetMathLibrary.Vector_Distance` _returnvalue (`self.PrevLocation`)))
  (set `self.PrevLocation` _returnvalue))

(fn `UserConstructionScript`)