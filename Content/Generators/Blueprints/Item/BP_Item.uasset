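; BP_Item is an item actor that shows its item class through a W_SimpleItemUI label taken from its preview widget component.
; SetupItemInformation stores the class and fills the label with index and system name.
; BeginPlay polls until that widget is valid, links it to the actor, moves it onto the shared W_ItemCanvas and hides the component.
; GenerateAffixes only picks a weighted index; class-roll, impulse and positioning logic sits unwired.
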(event `self.ReceiveBeginPlay`
  (bind _as_w_simple_item_ui (`self.As W Simple Item UI`))
  (bind _foundwidgets (`WidgetBlueprintLibrary.GetAllWidgetsOfClass` "/Game/Generators/W_ItemCanvas.W_ItemCanvas_C"))
  (set `self.General CAnvas` (`|GetArrayItem` _foundwidgets))
  (`/Engine/EditorBlueprintResources/StandardMacros.IsValid` _as_w_simple_item_ui :!label _label
    (:`Is Valid`
      (`/Game/Generators/W_SimpleItemUI.Set My Item Object` (`self.As W Simple Item UI`) self)
      (`/Game/Generators/W_ItemCanvas.Add Child To Canvas and Update Position` (`self.General CAnvas`) _as_w_simple_item_ui)
      (`SceneComponent.SetVisibility` (`self.ITemPreview`) false false))
    (:`Is Not Valid`
      (`KismetSystemLibrary.Delay` 0.0)
      (goto _label))))

(event `self.ReceiveTick`
  (params (DeltaSeconds :type "Float (single-precision)")))

(fn `Generate Affixes`
  (locals (Values :type "Array of Float (double-precision)") (Summ :type "Float (double-precision)" :default 0.0) (`Local Index` :type Integer :default 0))
  (bind _values (`/Game/Generators/Blueprints/Item/Items_FL.Get Affix Weights` (`/Game/Generators/Data/ItemClass/PDA_ItemBaseClass.GetSystem Name` (`self.Item Class`))))
  (set `local.Values` _values)
  (bind _summ (`/Game/Generators/Blueprints/Item/Items_FL.Get Affix Weights Summ` (`/Game/Generators/Data/ItemClass/PDA_ItemBaseClass.GetSystem Name` (`self.Item Class`))))
  (set `local.Summ` _summ)
  (bind _array_index (`/Game/Generators/Blueprints/Item/Items_FL.Get Index  from Weight` (`local.Values`) (`local.Summ`)))
  (set `local.Local Index` _array_index))

(fn `Setup Item Information`
  (params (`Item Class` :type "/Game/Generators/Data/ItemClass/PDA_ItemBaseClass Object Reference"))
  (bind _output_get (set `self.Item Class` `Item Class`))
  (bind _asw_simple_item_ui (cast `/Game/Generators/W_SimpleItemUI` (`WidgetComponent.GetUserWidgetObject` (`self.ITemPreview`))))
  (set `self.As W Simple Item UI` _asw_simple_item_ui)
  (`/Game/Generators/W_SimpleItemUI.Setup Item Info` _asw_simple_item_ui (`|FormatText` "{1}{2}" (`self.Array Index`) (`KismetTextLibrary.Conv_NameToText` (`/Game/Generators/Data/ItemClass/PDA_ItemBaseClass.System Name` _output_get))))
  (set `/Game/Generators/W_SimpleItemUI.Item Class` (`self.Item Class`) (`self.As W Simple Item UI`)))

(fn `UserConstructionScript`)