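; Blueprint function library of weighted-random helpers for item generation.
; It reads item classes, weights and tags from DT_ItemClassWeight and affix weights from DT_AffixRules, returning weight arrays, sums and tag-filtered rows.
; A cumulative-sum roll turns weights into a random index, which can resolve to an item class by row order.
; Tag filtering also returns row names, so weights can be gathered for just that subset.
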(fn `Filter Items By Tag`
  (params (Tags :type "GameplayTagContainer Structure"))
  (returns (`Filtered Items1` :type "Array of /Game/Generators/Data/ItemClass/ItemClassWeight Structure") (`Filtered Row Names1` :type "Array of Name"))
  (locals (`Filtered Items` :type "Array of /Game/Generators/Data/ItemClass/ItemClassWeight Structure") (`Filtered Row Names` :type "Array of Name"))
  (bind _outrownames (`DataTableFunctionLibrary.GetDataTableRowNames` "/Game/Generators/Data/ItemClass/DT_ItemClassWeight.DT_ItemClassWeight"))
  (for _array_element _outrownames
    (bind _returnvalue (`|GetDataTableRow` "/Game/Generators/Data/ItemClass/DT_ItemClassWeight.DT_ItemClassWeight" _array_element)
      (:`then`
        (if (`BlueprintGameplayTagLibrary.HasAnyTags` Tags (`.ItemTags_8_6FA9852946D697165E592C9560682A23` (break `/Game/Generators/Data/ItemClass/ItemClassWeight` _returnvalue)))
          (`KismetArrayLibrary.Array_Add` (`local.Filtered Items`) _returnvalue)
          (`KismetArrayLibrary.Array_Add` (`local.Filtered Row Names`) _array_element)))))
  (return (`local.Filtered Items`) (`local.Filtered Row Names`)))

(fn `Get Affix Weights`
  (params (RowName :type Name))
  (returns (Values :type "Array of Float (double-precision)"))
  (bind _returnvalue (`|GetDataTableRow` "/Game/Generators/Data/ItemAffixRules/DT_AffixRules.DT_AffixRules" RowName)
    (:`then`
      (bind _values (`BlueprintMapLibrary.Map_Values` (`.Affixes_7_C642C6FF4D119C11FC9519B83E0455BE` (break `/Game/Generators/Data/ItemAffixRules/ItemClassAffixRules_Struct` _returnvalue))))
      (return _values))))

(fn `Get Affix Weights Summ`
  (params (RowName :type Name))
  (returns (Summ :type "Float (double-precision)"))
  (locals (NewLocalVar_0 :type "Float (double-precision)" :default 1.0))
  (bind _returnvalue (`|GetDataTableRow` "/Game/Generators/Data/ItemAffixRules/DT_AffixRules.DT_AffixRules" RowName)
    (:`then`
      (bind _values (`BlueprintMapLibrary.Map_Values` (`.Affixes_7_C642C6FF4D119C11FC9519B83E0455BE` (break `/Game/Generators/Data/ItemAffixRules/ItemClassAffixRules_Struct` _returnvalue))))
      (for _array_element _values
        (set `local.NewLocalVar_0` (+ _array_element (`local.NewLocalVar_0`))))
      (return (`local.NewLocalVar_0`)))))

(fn `Get Index  from Weight`
  (params (Weights :type "Array of Float (double-precision)") (`Weight Summ` :type "Float (double-precision)"))
  (returns (`Array Index` :type Integer))
  (locals (sum :type "Float (double-precision)") (`Result Value` :type "Float (double-precision)" :default 0.0))
  (set `local.Result Value` (`KismetMathLibrary.RandomFloatInRange` 0.0 `Weight Summ`))
  (for (_array_element _array_index) Weights
    (bind _output_get (set `local.sum` (+ (`local.sum`) _array_element)))
    (if (>= _output_get (`local.Result Value`))
      (return _array_index))))

(fn `Get Item Class from Index`
  (params (Index :type Integer))
  (returns (`Item Class` :type "/Game/Generators/Data/ItemClass/PDA_ItemBaseClass Object Reference") (Success :type Boolean))
  (bind _outrownames (`DataTableFunctionLibrary.GetDataTableRowNames` "/Game/Generators/Data/ItemClass/DT_ItemClassWeight.DT_ItemClassWeight"))
  (bind _returnvalue (`|GetDataTableRow` "/Game/Generators/Data/ItemClass/DT_ItemClassWeight.DT_ItemClassWeight" (`|GetArrayItem` _outrownames Index))
    (:`then`
      (bind _itemclass (break `/Game/Generators/Data/ItemClass/ItemClassWeight` _returnvalue))
      (`/Engine/EditorBlueprintResources/StandardMacros.IsValid` _itemclass
        (:`Is Valid`
          (return _itemclass true))
        (:`Is Not Valid`
          (return null false))))))

(fn `Get Item Class Weights`
  (returns (Weights :type "Array of Float (double-precision)"))
  (locals (`Weight Array 11` :type Boolean) (Arr :type "Array of Float (double-precision)"))
  (bind _outrownames (`DataTableFunctionLibrary.GetDataTableRowNames` "/Game/Generators/Data/ItemClass/DT_ItemClassWeight.DT_ItemClassWeight"))
  (for _array_element _outrownames
    (bind _returnvalue (`|GetDataTableRow` "/Game/Generators/Data/ItemClass/DT_ItemClassWeight.DT_ItemClassWeight" _array_element)
      (:`then`
        (`KismetArrayLibrary.Array_Add` (`local.Arr`) (`.Weight_5_F19BACB641E8232CBBD02FBB81A24737` (break `/Game/Generators/Data/ItemClass/ItemClassWeight` _returnvalue))))))
  (return (`local.Arr`)))

(fn `Get Item Class Weights by Name`
  (params (Array :type "Array of Name"))
  (returns (Weights :type "Array of Float (double-precision)"))
  (locals (`Weight Array 11` :type Boolean) (Arr :type "Array of Float (double-precision)"))
  (for _array_element Array
    (bind _returnvalue (`|GetDataTableRow` "/Game/Generators/Data/ItemClass/DT_ItemClassWeight.DT_ItemClassWeight" _array_element)
      (:`then`
        (`KismetArrayLibrary.Array_Add` (`local.Arr`) (`.Weight_5_F19BACB641E8232CBBD02FBB81A24737` (break `/Game/Generators/Data/ItemClass/ItemClassWeight` _returnvalue))))))
  (return (`local.Arr`)))

(fn `Get Item Class Weights Summ`
  (returns (`Weights Summ` :type "Float (double-precision)"))
  (locals (`Weight Array 11` :type Boolean) (Arr :type "Array of Float (double-precision)") (Summ :type "Float (double-precision)" :default 1.0))
  (bind _outrownames (`DataTableFunctionLibrary.GetDataTableRowNames` "/Game/Generators/Data/ItemClass/DT_ItemClassWeight.DT_ItemClassWeight"))
  (for _array_element _outrownames
    (bind _returnvalue (`|GetDataTableRow` "/Game/Generators/Data/ItemClass/DT_ItemClassWeight.DT_ItemClassWeight" _array_element)
      (:`then`
        (set `local.Summ` (+ (`.Weight_5_F19BACB641E8232CBBD02FBB81A24737` (break `/Game/Generators/Data/ItemClass/ItemClassWeight` _returnvalue)) (`local.Summ`))))))
  (return (`local.Summ`)))

(fn `Summ Array`
  (params (Array :type "Array of Float (double-precision)"))
  (returns (Summ :type "Float (double-precision)"))
  (locals (`Arr Summ` :type "Float (double-precision)" :default 0.0))
  (for _array_element Array
    (set `local.Arr Summ` (+ _array_element (`local.Arr Summ`))))
  (return (`local.Arr Summ`)))